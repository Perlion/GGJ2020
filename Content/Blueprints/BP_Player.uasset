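; Player character that moves along its forward axis, jumps, interacts with nearby actors and carries one gear, which changes jump height and shows an indicator plane.
; Each Tick reapplies gear state, creating a new dynamic material while held, and highlights an available actor in PickupRange for Select via interface messages.
; A child animation actor handles jump and landing, with a short delay before jumping.
; Timelines drive a screen-plane fade in and out.
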(event `AccomidateGear`
  (bind _plane (`self.Plane`))
  (`self.Gear`
    (:`then`
      (set `CharacterMovementComponent.JumpZVelocity` (`self.JumpHeightWithGear`) (`self.CharacterMovement`))
      (`SceneComponent.SetHiddenInGame` _plane false false)
      (bind _returnvalue (`PrimitiveComponent.CreateDynamicMaterialInstance` _plane 0 (`PrimitiveComponent.GetMaterial` _plane 0) "None"))
      (`MaterialInstanceDynamic.SetScalarParameterValue` _returnvalue "Emissive" 0.0)
      (`MaterialInstanceDynamic.SetVectorParameterValue` :`self` _returnvalue :`ParameterName` "ColorChange"))
    (:`else`
      (set `CharacterMovementComponent.JumpZVelocity` (`self.DefaultJumpZ`) (`self.CharacterMovement`))
      (`SceneComponent.SetHiddenInGame` (`self.Plane`) true false))))

(event `InputAxis|MoveHorizontal`
  (params (AxisValue :type "Float (single-precision)"))
  (`self.AddMovementInput` (`self.GetActorForwardVector`) (* AxisValue (`self.MovementSpeed`))))

(event `self.ReceiveTick`
  (params (DeltaSeconds :type "Float (single-precision)"))
  (`self.AccomidateGear`)
  (`self.FindOverlappingActorToHighlight` (`PrimitiveComponent.GetOverlappingActors` (`self.PickupRange`) null)))

(event `Show Gear Preview`
  (bind _plane1 (`self.Plane1`))
  (`SceneComponent.SetHiddenInGame` _plane1 false false)
  (bind _returnvalue (`PrimitiveComponent.CreateDynamicMaterialInstance` _plane1 0 (`PrimitiveComponent.GetMaterial` _plane1 0) "None"))
  (`MaterialInstanceDynamic.SetScalarParameterValue` _returnvalue "Emissive" 30.0)
  (`MaterialInstanceDynamic.SetVectorParameterValue` _returnvalue "None" (struct :`R` 1.0 :`G` 0.537255 :`A` 1.0)))

(event `self.ReceiveBeginPlay`
  (`self.FadeIn`))

(event `InputAction|Select`
  (params (Key :type "Key Structure"))
  (:`Pressed`
    (message `/Game/Blueprints/ParentClasses/BPI_Interaction.Interact` (`self.OverlappingActor`) self)))

(event `FadeOut`
  (bind _screenfadeplane (`self.ScreenFadePlane`))
  (bind _returnvalue (`PrimitiveComponent.CreateDynamicMaterialInstance` _screenfadeplane 0 (`PrimitiveComponent.GetMaterial` _screenfadeplane 0) "None"))
  (`MaterialInstanceDynamic.SetScalarParameterValue` _returnvalue "None" 0.0)
  (bind (_direction _fadetime) (`Timeline|FadeOutTimeline` :!via `PlayFromStart`)
    (:`Update`
      (`MaterialInstanceDynamic.SetScalarParameterValue` _returnvalue "Opacity" _fadetime))
    (:`Finished`
      (`self.FadeOutFinished`))))

(event `Hide Gear Preview`
  (bind _plane1 (`self.Plane1`))
  (`SceneComponent.SetHiddenInGame` _plane1 true false)
  (bind _returnvalue (`PrimitiveComponent.CreateDynamicMaterialInstance` _plane1 0 (`PrimitiveComponent.GetMaterial` _plane1 0) "None"))
  (`MaterialInstanceDynamic.SetScalarParameterValue` _returnvalue "Emissive" 0.0)
  (`MaterialInstanceDynamic.SetVectorParameterValue` :`self` _returnvalue :`ParameterName` "ColorChange"))

(event `FadeIn`
  (bind _screenfadeplane (`self.ScreenFadePlane`))
  (bind _returnvalue (`PrimitiveComponent.CreateDynamicMaterialInstance` _screenfadeplane 0 (`PrimitiveComponent.GetMaterial` _screenfadeplane 0) "None"))
  (`MaterialInstanceDynamic.SetScalarParameterValue` _returnvalue "None" 1.0)
  (bind (_direction _fadetime) (`Timeline|FadeTimeline` :!via `ReverseFromEnd`)
    (:`Update`
      (`MaterialInstanceDynamic.SetScalarParameterValue` _returnvalue "Opacity" _fadetime))))

(event `InputAction|Jump`
  (params (Key :type "Key Structure"))
  (:`Pressed`
    (bind _asbp_player_animation (cast `/Game/Blueprints/BP_Player_Animation` (`ChildActorComponent.ChildActor` (`self.BP_Player_Animation`))))
    (`/Game/Blueprints/BP_Player_Animation.StartJump` _asbp_player_animation)
    (`KismetSystemLibrary.Delay` 0.07)
    (`self.Jump`)))

(event `RemoveGear`
  (set `self.Gear` null))

(event `AddGear`
  (params (Gear :type "/Game/Blueprints/BP_Gear Object Reference"))
  (bind _output_get (set `self.Gear` Gear))
  (`self.K2_SetActorLocation` _output_get (0.0 0.0 -1000.0) false false))

(event `self.OnLanded`
  (params (Hit :type "HitResult Structure (by ref)"))
  (bind _asbp_player_animation (cast `/Game/Blueprints/BP_Player_Animation` (`ChildActorComponent.ChildActor` (`self.BP_Player_Animation`))))
  (`/Game/Blueprints/BP_Player_Animation.LandingAnimation` _asbp_player_animation))

(fn `AvaliableForInteract`
  (returns (CanBeInteracted :type Boolean))
  (return false))

(fn `FindOverlappingActorToHighlight`
  (params (Array :type "Array of Actor Object Reference"))
  (locals (FoundActorToInteract :type Boolean :default false))
  (bind _overlappingactor (`self.OverlappingActor`))
  (for _array_element Array
    (if (not (`local.FoundActorToInteract`))
      (bind _canbeinteracted (message `/Game/Blueprints/ParentClasses/BPI_Interaction.AvaliableForInteract` _array_element))
      (if _canbeinteracted
        (set `local.FoundActorToInteract` true)
        (if (!= _array_element (`self.OverlappingActor`))
          (message `/Game/Blueprints/ParentClasses/BPI_Interaction.Unhighlight` (`self.OverlappingActor`))
          (set `self.OverlappingActor` _array_element)
          (else
            (message `/Game/Blueprints/ParentClasses/BPI_Interaction.Highlight` (`self.OverlappingActor`)))))))
  (if (`local.FoundActorToInteract`)
    (message `/Game/Blueprints/ParentClasses/BPI_Interaction.Highlight` _overlappingactor)
    (else
      (message `/Game/Blueprints/ParentClasses/BPI_Interaction.Unhighlight` _overlappingactor)
      (set `self.OverlappingActor` null))))

(fn `UserConstructionScript`
  (set `self.DefaultJumpZ` (`CharacterMovementComponent.JumpZVelocity` (`self.CharacterMovement`))))