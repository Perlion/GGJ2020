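; BP_Active_Actor_Parent is a base actor for mechanisms whose looping sound depends on whether a gear sits in their GearHolder.
; BeginPlay spawns the loop at world origin and stores the audio component.
; Tick checks the holder's GearReference, unpausing the sound when a gear is present and pausing it otherwise.
; Two DoOnce gates reset each other, so each switch fires only when the gear state changes.
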(event `self.ReceiveBeginPlay`
  (bind _returnvalue (`GameplayStatics.SpawnSoundAtLocation` (`self.LoopingMechanismSound`) (0.0 0.0 0.0) (struct) 1.0 1.0 0.0 null null))
  (set `self.InGameLoopingSound` _returnvalue))

(event `self.ReceiveTick`
  (params (DeltaSeconds :type "Float (single-precision)"))
  (bind _ingameloopingsound (`self.InGameLoopingSound`))
  (bind _gearholder (`self.GearHolder`)
    (:`then`
      (`/Game/Blueprints/BP_GearHolder.GearReference` _gearholder
        (:`then`
          (`/Engine/EditorBlueprintResources/StandardMacros.DoOnce` false :!label _label
            (:`Completed`
              (`AudioComponent.SetPaused` _ingameloopingsound false)
              (`self.ResetStopSound`))))
        (:`else`
          (`/Engine/EditorBlueprintResources/StandardMacros.DoOnce` false :!label _label_2
            (:`Completed`
              (`AudioComponent.SetPaused` _ingameloopingsound true)
              (`self.ResetStartSound`))))))
    (:`else`)))

(event `ResetStartSound`
  (goto _label :!via `Reset`))

(event `ResetStopSound`
  (goto _label_2 :!via `Reset`))

(fn `UserConstructionScript`)