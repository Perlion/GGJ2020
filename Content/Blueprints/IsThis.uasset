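; IsThis is a Blueprint with no working behavior, and its purpose in the game is not evident.
; Its event graph holds only disconnected trees of boolean AND and OR nodes on constant false inputs, with no events and nothing reading the results.
; The construction script is empty.
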(fn `UserConstructionScript`)