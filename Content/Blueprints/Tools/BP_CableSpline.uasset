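; Spline-based cable actor that lights up or goes dark according to the state of a referenced lever.
; The construction script lays spline mesh segments at fixed section lengths, skipping any whose end-to-end distance falls short of that length minus a deformation margin.
; Tick compares the lever with ActiveWhenLeverUp, using two cross-resetting DoOnce gates to update emissive and color through dynamic materials only on state changes.
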(event `self.ReceiveBeginPlay`)

(event `self.ReceiveTick`
  (params (DeltaSeconds :type "Float (single-precision)"))
  (bind _leverreference (`self.LeverReference`)
    (:`then`
      (if (== (`/Game/Blueprints/BP_Lever.leverUp` _leverreference) (`self.ActiveWhenLeverUp?`))
        (`/Engine/EditorBlueprintResources/StandardMacros.DoOnce` false :!label _label
          (:`Completed`
            (`self.AdjustEmissive` 1.0)
            (`self.ResetOff`)))
        (else
          (`/Engine/EditorBlueprintResources/StandardMacros.DoOnce` false :!label _label_2
            (:`Completed`
              (`self.AdjustEmissive` 0.0)
              (`self.ResetOn`))))))
    (:`else`)))

(event `ResetOn`
  (goto _label :!via `Reset`))

(event `ResetOff`
  (goto _label_2 :!via `Reset`))

(fn `AdjustEmissive`
  (params (Value :type "Float (double-precision)"))
  (for _array_element (`self.K2_GetComponentsByClass` "/Script/Engine.SplineMeshComponent")
    (bind _returnvalue (`PrimitiveComponent.CreateDynamicMaterialInstance` _array_element 0 (`PrimitiveComponent.GetMaterial` _array_element 0) "None"))
    (`MaterialInstanceDynamic.SetScalarParameterValue` _returnvalue "Emissive" (* Value 75.0))
    (`MaterialInstanceDynamic.SetVectorParameterValue` _returnvalue "ColorChange" (* (struct :`R` 0.591146 :`G` 0.485572 :`A` 1.0) Value))))

(fn `UserConstructionScript`
  (bind _spline (`self.Spline`))
  (bind _spline_2 (`self.Spline`))
  (for _index (range (+ (`KismetMathLibrary.FTrunc` (/ (`SplineComponent.GetSplineLength` (`self.Spline`)) (`self.SectionLength`))) 1))
    (if (>= (`KismetMathLibrary.VSize` (- (`SplineComponent.GetLocationAtDistanceAlongSpline` (`self.Spline`) (* _index (`self.SectionLength`)) "Local") (`SplineComponent.GetLocationAtDistanceAlongSpline` (`self.Spline`) (* (+ _index 1) (`self.SectionLength`)) "Local"))) (- (`self.SectionLength`) (`self.DeformMagin`)))
      (bind _returnvalue (`AddComponent|NODE_AddSplineMeshComponent-1`))
      (`SceneComponent.K2_AttachToComponent` _returnvalue (`self.Spline`) "None" "KeepRelative" "KeepRelative" "KeepRelative" true)
      (bind _returnvalue_2 (* _index (`self.SectionLength`)))
      (bind _returnvalue_3 (* (+ _index 1) (`self.SectionLength`)))
      (`SplineMeshComponent.SetStartAndEnd` _returnvalue (`SplineComponent.GetLocationAtDistanceAlongSpline` _spline _returnvalue_2 "Local") (`SplineComponent.GetTangentAtDistanceAlongSpline` _spline _returnvalue_2 "Local") (`SplineComponent.GetLocationAtDistanceAlongSpline` _spline_2 _returnvalue_3 "Local") (`SplineComponent.GetTangentAtDistanceAlongSpline` _spline_2 _returnvalue_3 "Local") true))))