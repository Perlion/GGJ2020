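; BP_TileSet is a construction-time tool that builds a grid of tiles from one instanced static mesh.
; The construction script applies TileMaterial, then adds rotated instances over nested column and row loops, spaced by tile width and height along the Arrow's forward and right vectors.
; A separate AdjustEmissive function creates dynamic materials on SplineMeshComponents, not the tile instances, scaling their emissive and color-change parameters by the input value.
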(fn `AdjustEmissive`
  (params (Value :type "Float (double-precision)"))
  (for _array_element (`self.K2_GetComponentsByClass` "/Script/Engine.SplineMeshComponent")
    (bind _returnvalue (`PrimitiveComponent.CreateDynamicMaterialInstance` _array_element 0 (`PrimitiveComponent.GetMaterial` _array_element 0) "None"))
    (`MaterialInstanceDynamic.SetScalarParameterValue` _returnvalue "Emissive" (* Value 75.0))
    (`MaterialInstanceDynamic.SetVectorParameterValue` _returnvalue "ColorChange" (* (struct :`R` 0.591146 :`G` 0.485572 :`A` 1.0) Value))))

(fn `UserConstructionScript`
  (bind _arrow (`self.Arrow`))
  (`PrimitiveComponent.SetMaterial` (`self.InstancedStaticMesh`) 0 (`self.TileMaterial`))
  (for _index (range (+ (`self.NumCollums`) 1))
    (for _index_2 (range (+ (`self.NumRows`) 1))
      (`InstancedStaticMeshComponent.AddInstance` (`self.InstancedStaticMesh`) (`KismetMathLibrary.MakeTransform` (+ (* (* (`SceneComponent.GetForwardVector` _arrow) (`self.TileWidth`)) _index_2) (* (* (`SceneComponent.GetRightVector` _arrow) (`self.TileHeight`)) _index)) (struct :`Roll` 90.0))))))