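; BP_Lever is an interactable lever that is always available for interaction and toggles between up and down.
; Interact flips LeverUp and snaps Scene1 to the world rotation of the SceneUp or SceneDown reference component; the construction script applies the initial pose.
; Highlight and Unhighlight toggle an emissive glow on Plane1 through dynamic material instances created on each call.
; The switch sound and highlight tint nodes are disconnected.
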(event `/Game/Blueprints/ParentClasses/BPI_Interaction.Unhighlight`
  (`self.HidePlacementIcon`))

(event `HidePlacementIcon`
  (bind _plane1 (`self.Plane1`))
  (bind _returnvalue (`PrimitiveComponent.CreateDynamicMaterialInstance` _plane1 0 (`PrimitiveComponent.GetMaterial` _plane1 0) "None"))
  (`MaterialInstanceDynamic.SetVectorParameterValue` _returnvalue "ColorChange" (struct :`A` 1.0))
  (`MaterialInstanceDynamic.SetScalarParameterValue` _returnvalue "Emissive" 0.0))

(event `/Game/Blueprints/ParentClasses/BPI_Interaction.Highlight`
  (`self.DisplayPlacementIcon`))

(event `DisplayPlacementIcon`
  (bind _plane1 (`self.Plane1`))
  (bind _returnvalue (`PrimitiveComponent.CreateDynamicMaterialInstance` _plane1 0 (`PrimitiveComponent.GetMaterial` _plane1 0) "None"))
  (`MaterialInstanceDynamic.SetScalarParameterValue` _returnvalue "Emissive" 30.0))

(event `/Game/Blueprints/ParentClasses/BPI_Interaction.Interact`
  (params (Player :type "/Game/Blueprints/BP_Player Object Reference"))
  (`self.FlipLever`))

(event `FlipLever`
  (if (`self.leverUp`)
    (set `self.leverUp` false)
    (`SceneComponent.K2_SetWorldRotation` (`self.Scene1`) (`SceneComponent.K2_GetComponentRotation` (`self.SceneDown`)) false false)
    (else
      (set `self.leverUp` true)
      (`SceneComponent.K2_SetWorldRotation` (`self.Scene1`) (`SceneComponent.K2_GetComponentRotation` (`self.SceneUp`)) false false))))

(fn `AvaliableForInteract`
  (returns (CanBeInteracted :type Boolean))
  (return true))

(fn `UserConstructionScript`
  (`parent.UserConstructionScript`)
  (if (`self.leverUp`)
    (`SceneComponent.K2_SetWorldRotation` (`self.Scene1`) (`SceneComponent.K2_GetComponentRotation` (`self.SceneUp`)) false false)
    (else
      (`SceneComponent.K2_SetWorldRotation` (`self.Scene1`) (`SceneComponent.K2_GetComponentRotation` (`self.SceneDown`)) false false))))