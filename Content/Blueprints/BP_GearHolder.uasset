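; BP_GearHolder is an interactable socket actor that holds a gear and tracks whether it should be turning.
; Interacting while the player carries a gear places it after a delay, linking it to the holder, snapping it to a right-vector offset and removing it from the player.
; An optional preassigned gear is placed on BeginPlay.
; Tick sets the turning flag whenever a gear is held, gated by an optional lever's on state.
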(event `self.ReceiveBeginPlay`
  (bind _gearreference (`self.GearReference`)
    (:`then`
      (`self.PlaceGearInHolder` self _gearreference))
    (:`else`)))

(event `ReomveGearFromHolder`
  (set `self.GearReference` null))

(event `self.ReceiveTick`
  (params (DeltaSeconds :type "Float (single-precision)"))
  (`self.GearReference`
    (:`then`
      (bind _leverreference (`self.leverReference`)
        (:`then`
          (if (`/Game/Blueprints/BP_Lever.leverOn` _leverreference)
            (set `self.isGearTurning` true)
            (else
              (set `self.isGearTurning` false))))
        (:`else`
          (set `self.isGearTurning` true))))
    (:`else`
      (set `self.isGearTurning` false))))

(event `PlaceGearInHolder`
  (params (GearToPlace :type "/Game/Blueprints/BP_Gear Object Reference"))
  (bind (_returnvalue_location _returnvalue_rotation) (`KismetMathLibrary.BreakTransform` (`self.GetTransform`)))
  (bind _output_get (set `self.GearReference` GearToPlace))
  (set `/Game/Blueprints/BP_Gear.GearHolder` self _output_get)
  (`self.K2_SetActorTransform` _output_get (`KismetMathLibrary.MakeTransform` (+ _returnvalue_location (* (`self.GetActorRightVector`) 10.0)) _returnvalue_rotation) false false))

(event `/Game/Blueprints/BPI_Interaction.Interact`
  (params (Player :type "/Game/Blueprints/BP_Player Object Reference"))
  (bind _gear (`/Game/Blueprints/BP_Player.Gear` Player)
    (:`then`
      (`KismetSystemLibrary.Delay` (`self.placeGearDelay`))
      (`self.PlaceGearInHolder` _gear)
      (`/Game/Blueprints/BP_Player.RemoveGear` Player))
    (:`else`)))

(fn `UserConstructionScript`)