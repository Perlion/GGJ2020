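; BP_Gear is a pickup gear that a player can carry and that can sit in a gear holder.
; Each tick it rotates on pitch at RotationRate while its holder reports the gear is turning.
; On Interact, if the player carries no gear, it detaches from any holder after a placement sound and short delay, then passes itself to the player via AddGear.
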(event `self.ReceiveTick`
  (params (DeltaSeconds :type "Float (single-precision)"))
  (bind _gearholder (`self.GearHolder`)
    (:`then`
      (if (`/Game/Blueprints/BP_GearHolder.isGearTurning` _gearholder)
        (`self.K2_AddActorLocalRotation` (`KismetMathLibrary.MakeRotator` 0.0 (`self.RotationRate`)))))
    (:`else`)))

(event `/Game/Blueprints/BPI_Interaction.Interact`
  (params (Player :type "/Game/Blueprints/BP_Player Object Reference"))
  (`/Game/Blueprints/BP_Player.Gear` Player
    (:`then`)
    (:`else`
      (bind _gearholder (`self.GearHolder`)
        (:`then`
          (`GameplayStatics.PlaySound2D` "/Game/Sounds/SoundCues/GearPlace_Cue.GearPlace_Cue" 1.0 1.0 0.0 null null)
          (`KismetSystemLibrary.Delay` (`self.pickupGearDelay`))
          (`/Game/Blueprints/BP_GearHolder.ReomveGearFromHolder` _gearholder)
          (set `self.GearHolder` null))
        (:`else`
          _))
      (`/Game/Blueprints/BP_Player.AddGear` Player self))))

(fn `UserConstructionScript`)