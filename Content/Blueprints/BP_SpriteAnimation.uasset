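; BP_SpriteAnimation plays a looping flipbook animation on a Plane component by swapping textures at FramesPerSecond.
; BeginPlay sets a timer on DoAnimationLoop, which writes the current SpriteAnimation entry to the "Texture" parameter of the plane's dynamic material instance.
; CurrentFrame increments each step, with modulo indexing to wrap the array.
; Each step also sets the looping timer again, so the delay follows the current FramesPerSecond.
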(event `self.ReceiveBeginPlay`
  (`parent.ReceiveBeginPlay`)
  (`KismetSystemLibrary.K2_SetTimerDelegate` (delegate `DoAnimationLoop`) (/ 1.0 (`self.FramesPerSecond`)) true :!label _label))

(event `DoAnimationLoop`
  (bind _plane (`self.Plane`))
  (bind _returnvalue (`PrimitiveComponent.CreateDynamicMaterialInstance` _plane 0 (`PrimitiveComponent.GetMaterial` _plane 0) "None"))
  (`MaterialInstanceDynamic.SetTextureParameterValue` _returnvalue "Texture" (`|GetArrayItem` (`self.SpriteAnimation`) (mod (`self.CurrentFrame`) (`KismetArrayLibrary.Array_Length` (`self.SpriteAnimation`)))))
  (`/Engine/EditorBlueprintResources/StandardMacros.IncrementInt` (`self.CurrentFrame`)
    (:`  `
      (goto _label))))

(fn `UserConstructionScript`
  (`parent.UserConstructionScript`))