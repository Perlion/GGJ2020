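; Gear-activated piston that slides back and forth along its Arrow's forward axis while the linked GearHolder's gear turns.
; Tick polls the gear and uses two cross-resetting DoOnce gates to start or stop movement.
; A timeline, rate-scaled by stroke duration, lerps the scene component, then flips direction and repeats after a delay.
; Finishing a push launches an overlapping player with an impulse; sound cues accompany strokes.
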(event `InterpolateBetweenPoints`
  (params (A :type "Vector Structure") (B :type "Float (double-precision)") (Scale :type "Float (double-precision)") (DelayBeforeStartingAgain :type "Float (double-precision)"))
  (`TimelineComponent.SetPlayRate` (`self.Timeline_0`) (/ 1.0 B))
  (set `self.ActorStartLocation` (`SceneComponent.K2_GetComponentLocation` (`self.Scene`)))
  (bind (_direction _time) (`Timeline|Timeline_0` :!via `PlayFromStart` :!label _label)
    (:`Update`
      (`SceneComponent.K2_SetWorldLocation` (`self.Scene`) (`self.FindNextPointToMoveTo` _time A Scale) false false))
    (:`Finished`
      (if (`self.isRetracting`)
        (`GameplayStatics.SpawnSoundAtLocation` "/Game/Sounds/SoundCues/PistonLower_Cue.PistonLower_Cue" (`self.K2_GetActorLocation`) (struct) 1.0 1.0 0.0 null null))
      (set `self.isRetracting` (not (`self.isRetracting`)))
      (if (`PrimitiveComponent.IsOverlappingActor` (`self.Box`) (`GameplayStatics.GetPlayerPawn` 0))
        (`self.ApplyForceToPlayer`))
      (`KismetSystemLibrary.Delay` DelayBeforeStartingAgain)
      (if (`/Game/Blueprints/BP_GearHolder.isGearTurning` (`self.GearHolder`))
        (`self.StartPlatformMove`)))))

(event `StopPlatformMove`
  (goto _label :!via `Stop`))

(event `StartPlatformMove`
  (if (`self.isRetracting`)
    (`self.InterpolateBetweenPoints` (`self.PointB`) (`self.TimeToResetPiston`) -1.0 (`self.TimeToWaitBeforePush`))
    (else
      (`self.InterpolateBetweenPoints` (`self.PointA`) (`self.TimeToLaunchPiston`) 1.0 (`self.TimeToWaitAfterPush`))
      (`GameplayStatics.SpawnSoundAtLocation` "/Game/Sounds/SoundCues/piston_Cue.piston_Cue" (`self.K2_GetActorLocation`) (struct) 1.0 1.0 0.0 null null))))

(event `self.ReceiveTick`
  (params (DeltaSeconds :type "Float (single-precision)"))
  (if (`/Game/Blueprints/BP_GearHolder.isGearTurning` (`self.GearHolder`))
    (`/Engine/EditorBlueprintResources/StandardMacros.DoOnce` false :!label _label_2
      (:`Completed`
        (`self.ResetStop`)
        (`self.StartPlatformMove`)))
    (else
      (`/Engine/EditorBlueprintResources/StandardMacros.DoOnce` false :!label _label_3
        (:`Completed`
          (`self.ResetStart`)
          (`self.StopPlatformMove`))))))

(event `ResetStart`
  (goto _label_2 :!via `Reset`))

(event `ResetStop`
  (goto _label_3 :!via `Reset`))

(fn `ApplyForceToPlayer`
  (if (`self.isRetracting`)
    (bind _asbp_player (cast `/Game/Blueprints/BP_Player` (`GameplayStatics.GetPlayerPawn` 0)))
    (`CharacterMovementComponent.AddImpulse` (`Character.CharacterMovement` _asbp_player) (* (`SceneComponent.GetForwardVector` (`self.Arrow`)) (`self.PushForce`)) true)))

(fn `FindNextPointToMoveTo`
  (params (Alpha :type "Float (double-precision)") (A :type "Vector Structure") (B :type "Float (double-precision)"))
  (returns (ReturnValue :type "Vector Structure"))
  (return (`KismetMathLibrary.VLerp` (`self.ActorStartLocation`) (+ (* (`SceneComponent.GetForwardVector` (`self.Arrow`)) (* (`KismetMathLibrary.VSize` A) B)) (`self.K2_GetActorLocation`)) Alpha)))

(fn `UserConstructionScript`
  (`parent.UserConstructionScript`)
  (if (`self.StartAtPointA?`)
    (`SceneComponent.K2_SetWorldLocation` (`self.Scene`) (+ (* (`SceneComponent.GetForwardVector` (`self.Arrow`)) (`KismetMathLibrary.VSize` (`self.PointA`))) (`self.K2_GetActorLocation`)) false false)
    (else
      (`SceneComponent.K2_SetWorldLocation` (`self.Scene`) (+ (`self.K2_GetActorLocation`) (* (* (`SceneComponent.GetForwardVector` (`self.Arrow`)) (`KismetMathLibrary.VSize` (`self.PointB`))) -1.0)) false false))))