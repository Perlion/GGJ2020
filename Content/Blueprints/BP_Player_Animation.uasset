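; Player sprite animation actor that picks the sprite cycle and frame rate from the player pawn's movement.
; While cycling is enabled, Tick selects falling, walk or idle from the falling state and speed.
; StartJump and LandingAnimation pause cycling, play their one-shot cycle, then resume after a delay derived from cycle length and frame rate.
; ApplyDirectionScale mirrors the plane on X using the dot product of actor forward and pawn velocity.
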(event `LandingAnimation`
  (bind _postjumpcycle (`self.PostJumpCycle`))
  (set `self.UsingAnimationCycle` false)
  (set `self.SpriteAnimation` _postjumpcycle)
  (bind _output_get (set `self.FramesPerSecond` 6.0))
  (`KismetSystemLibrary.Delay` (/ (`KismetMathLibrary.Conv_IntToDouble` (`KismetArrayLibrary.Array_Length` _postjumpcycle)) _output_get))
  (set `self.UsingAnimationCycle` true))

(event `StartJump`
  (bind _prejumpcycle (`self.PreJumpCycle`))
  (set `self.UsingAnimationCycle` false)
  (set `self.SpriteAnimation` _prejumpcycle)
  (bind _output_get (set `self.FramesPerSecond` 16.0))
  (`KismetSystemLibrary.Delay` (/ (`KismetMathLibrary.Conv_IntToDouble` (`KismetArrayLibrary.Array_Length` _prejumpcycle)) _output_get))
  (set `self.UsingAnimationCycle` true))

(event `self.ReceiveTick`
  (params (DeltaSeconds :type "Float (single-precision)"))
  (bind _returnvalue (`Pawn.GetMovementComponent` (`GameplayStatics.GetPlayerPawn` 0)))
  (if (`self.UsingAnimationCycle`)
    (`self.ApplyDirectionScale`)
    (if (`NavMovementComponent.IsFalling` _returnvalue)
      (set `self.SpriteAnimation` (`self.FallingCycle`))
      (elif (> (`KismetMathLibrary.VSize` (`MovementComponent.Velocity` _returnvalue)) 50.0)
        (set `self.SpriteAnimation` (`self.WalkCycle`))
        (set `self.FramesPerSecond` 12.0)
        (else
          (set `self.SpriteAnimation` (`self.IdleCycle`))
          (set `self.FramesPerSecond` 5.0))))))

(fn `ApplyDirectionScale`
  (bind _returnvalue (`KismetMathLibrary.FCeil` (`KismetMathLibrary.Dot_VectorVector` (`self.GetActorForwardVector`) (`KismetMathLibrary.Normal` (`self.GetVelocity` (`GameplayStatics.GetPlayerPawn` 0))))))
  (if (!= (`KismetMathLibrary.Conv_IntToDouble` _returnvalue) 0.0)
    (`SceneComponent.SetWorldScale3D` (`self.Plane`) (`KismetMathLibrary.MakeVector` (`KismetMathLibrary.FClamp` (`KismetMathLibrary.Conv_IntToDouble` _returnvalue) -1.0) 1.0 1.0))))

(fn `UserConstructionScript`
  (`parent.UserConstructionScript`))