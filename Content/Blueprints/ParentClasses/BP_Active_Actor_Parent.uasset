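; Parent actor for gear-driven mechanisms that plays a looping mechanism sound while its linked gear turns.
; BeginPlay spawns the attenuated loop at the actor's location and pauses it immediately.
; Tick polls GearHolder's IsGearTurning, firing Activated or Deactivated to unpause or pause the sound.
; Two DoOnce gates, each reset by the opposite state, limit those events to state changes.
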(event `self.ReceiveBeginPlay`
  (bind _returnvalue (`GameplayStatics.SpawnSoundAtLocation` (`self.LoopingMechanismSound`) (`self.K2_GetActorLocation`) (struct) 2.0 1.0 0.0 "/Game/Sounds/HearingFalloff.HearingFalloff" null))
  (bind _output_get (set `self.InGameLoopingSound` _returnvalue))
  (`AudioComponent.SetPaused` _output_get true))

(event `Activated`
  (`AudioComponent.SetPaused` (`self.InGameLoopingSound`) false)
  (`self.ResetStopSound`))

(event `self.ReceiveTick`
  (params (DeltaSeconds :type "Float (single-precision)"))
  (bind _gearholder (`self.GearHolder`)
    (:`then`
      (if (`/Game/Blueprints/BP_GearHolder.isGearTurning` _gearholder)
        (`/Engine/EditorBlueprintResources/StandardMacros.DoOnce` false :!label _label
          (:`Completed`
            (`self.Activated`)))
        (else
          (`/Engine/EditorBlueprintResources/StandardMacros.DoOnce` false :!label _label_2
            (:`Completed`
              (`self.Deactivated`))))))
    (:`else`)))

(event `Deactivated`
  (`AudioComponent.SetPaused` (`self.InGameLoopingSound`) true)
  (`self.ResetStartSound`))

(event `ResetStartSound`
  (goto _label :!via `Reset`))

(event `ResetStopSound`
  (goto _label_2 :!via `Reset`))

(fn `UserConstructionScript`)